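; Base character that moves along a spline, judging by its name a parent for other characters.
; BeginPlay sets the current speed to walk speed.
; AddMoviment zeroes the acceleration variable and advances the spline distance by speed, axis value and frame delta time.
; UpdateLocation places the actor at that distance in world space with rotation unwired; neither function is called here.
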(event EventBeginPlay
  (Variables|Default|SetCharacterSpeed (Variables|Default|GetWalkSpeed)))

(event Collision|EventActorBeginOverlap
  (params (OtherActor :type Actor%20Object%20Reference)))

(event EventTick
  (params (DeltaSeconds :type Float%20%28single-precision%29)))

(fn ConstructionScript)

(fn UpdateLocation
  (Transformation|SetActorLocationAndRotation (Spline|GetLocationatDistanceAlongSpline (Variables|/Game/Blueprints/Spline.Spline_C|GetSpline (Variables|Default|GetSplineRef)) (Variables|Default|GetDistanceAlongSpline) "World") "0, 0, 0"))

(fn AddMoviment
  (Variables|Default|SetPlayerAccelaration 0.0)
  (Variables|Default|SetDistanceAlongSpline (+ (Variables|Default|GetDistanceAlongSpline) (* (* (Variables|Default|GetCharacterSpeed) (Variables|Default|GetAxisValue)) (Utilities|Time|GetWorldDeltaSeconds)))))