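; SplineCharacter is a Blueprint, apparently a character, that travels along a referenced spline.
; Each Tick calls UpdateLocation and AddMoviment, whose bodies are not shown here.
; It then resets DistanceAlongSpline to zero when it nearly equals the spline's length, using a very tight tolerance, to loop back to the start.
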(event EventBeginPlay
  (|CallParentFunction) ; This node is disabled and will not be called.\nDrag off pins to build functionality.
)

(event EventTick
  (params (DeltaSeconds :type Float%20%28single-precision%29))
  (CallFunction|UpdateLocation)
  (CallFunction|AddMoviment)
  (if (Math|Float|NearlyEqual(Float) (Variables|Default|GetDistanceAlongSpline) (Spline|GetSplineLength (Variables|/Game/Blueprints/Spline.Spline_C|GetSpline (Variables|Default|GetSplineRef))) 1e-06)
    (Variables|Default|SetDistanceAlongSpline 0.0)))

(fn ConstructionScript
  (|CallParentFunction))