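; AI character Blueprint that wanders randomly around the navmesh.
; On BeginPlay it picks a random walk speed, then starts a walk loop.
; WalkEvent sends AIMoveTo to a random navigable point within WalkRadius of the current location, guarded by the NotWalking flag.
; Success or failure both wait a random delay, clear the flag and trigger the next walk.
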(event Custom|walk%20event
  (if (not (Variables|Default|GetNot%20Walking?))
    (AI|AIMoveTo self (.RandomLocation (Class|NavigationSystemV1|GetRandomPointinNavigableRadius (Transformation|GetActorLocation) (Variables|Default|Getwalk%20radius) 0 0)) 0 5.0 false
      (:then
        (Variables|Default|SetNot%20Walking? true))
      (:OnSuccess
        (Utilities|FlowControl|Delay (Math|Random|RandomFloatinRange 0.0 4.0) :!label _label)
        (Variables|Default|SetNot%20Walking? false)
        (CallFunction|WalkEvent))
      (:OnFail
        (goto _label)))))

(event EventBeginPlay
  (bind _output_get (Variables|Default|SetWalk%20Speed (Math|Random|RandomFloatinRange 1e+02 2e+02)))
  (Variables|/Script/Engine.CharacterMovementComponent|SetMaxWalkSpeed (Variables|Character|GetCharacterMovement) _output_get)
  (CallFunction|WalkEvent))

(fn ConstructionScript)