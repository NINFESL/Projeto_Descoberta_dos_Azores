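; SplineCharacter is a child Blueprint that moves along a referenced spline in a continuous loop.
; Each tick it calls the inherited UpdateLocationAndRotation and AddMovement functions to update its transform and movement.
; It then resets DistanceAlongSpline to zero when that distance comes within a small tolerance of the spline's length, restarting the path from the beginning.
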(event EventBeginPlay
  (|CallParentFunction))

(event EventTick
  (params (DeltaSeconds :type Float%20%28single-precision%29))
  ;[1 1 1] Call parent functions to update movements location adn rotation
  (CallFunction|UpdateLocationandRotation)
  (CallFunction|AddMovement)
  ;[1 1 1] Did we reach the end of the spline? If so reset distance along spline and start at zero
  (if (Math|Float|NearlyEqual(Float) (Variables|Default|GetDistanceAlongSpline) (Spline|GetSplineLength (Variables|/Game/Blueprint/Spline.Spline_C|GetSpline (Variables|Default|GetSplineRef))) 1e+01)
    (Variables|Default|SetDistanceAlongSpline 0.0)))

(fn ConstructionScript
  (|CallParentFunction))