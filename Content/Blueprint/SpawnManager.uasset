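; Spawn manager that populates every Spline actor in the level with AI-controlled characters at BeginPlay.
; It divides each spline's length by its character count and spawns characters at even intervals, aligned to the spline's location and rotation.
; Classes cycle through each spline's spawnable list using an index that is not reset between splines.
; Each character receives its spline reference and starting distance, then spawns its default controller.
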(event EventBeginPlay
  (bind _outactors (Actor|GetAllActorsOfClass "/Game/Blueprint/Spline.Spline_C"))
  (Variables|Default|SetSplinesRef _outactors)
  (CallFunction|SpawnNextSplineCharacter))

(fn ConstructionScript)

(fn SpawnNextSplineCharacter
  ;[1 1 1] For each spline in the level calculate how many characters on the spline based on the number of character on spline var
  (for _array_element (Variables|Default|GetSplinesRef)
    (bind _output_get (LocalVariables|SetCurrentSpline _array_element))
    (LocalVariables|SetSplineDivision (/ (Spline|GetSplineLength (Variables|/Game/Blueprint/Spline.Spline_C|GetSpline _output_get)) (Math|Conversions|ToFloat(Integer) (Variables|/Game/Blueprint/Spline.Spline_C|GetNumberOfCharactersOnSpline _output_get))))
    (for _index (range 1 (Variables|/Game/Blueprint/Spline.Spline_C|GetNumberOfCharactersOnSpline _output_get))
      ;[1 1 1] Spawn the character based on the current distance along the spline
      (bind _returnvalue (Game|SpawnActorfromClass (Utilities|Array|Get(acopy) (Variables|/Game/Blueprint/Spline.Spline_C|GetSpawnableSplineCharacters (LocalVariables|GetCurrentSpline)) (LocalVariables|GetSplineCharacterIndex)) (Math|Transform|MakeTransform (Spline|GetLocationatDistanceAlongSpline (Variables|/Game/Blueprint/Spline.Spline_C|GetSpline (LocalVariables|GetCurrentSpline)) (LocalVariables|GetCurrentDistance) "World") (Spline|GetRotationatDistanceAlongSpline (Variables|/Game/Blueprint/Spline.Spline_C|GetSpline (LocalVariables|GetCurrentSpline)) (LocalVariables|GetCurrentDistance) "World")) "AdjustIfPossibleButAlwaysSpawn" 0 0))
      ;[1 1 1] Initialise characters variables and spawn AI Controller
      (Variables|/Game/Blueprint/ParentCharacter.ParentCharacter_C|SetSplineRef _returnvalue (LocalVariables|GetCurrentSpline))
      (Variables|/Game/Blueprint/ParentCharacter.ParentCharacter_C|SetDistanceAlongSpline _returnvalue (LocalVariables|GetCurrentDistance))
      (Pawn|SpawnDefaultController _returnvalue)
      ;[1 1 1] Update distance along spline based on the divisions calculated
      (LocalVariables|SetCurrentDistance (+ (LocalVariables|GetCurrentDistance) (LocalVariables|GetSplineDivision)))
      ;[1 1 1] Who's the next character to spawn?
      (if (>= (LocalVariables|GetSplineCharacterIndex) (- (Utilities|Array|Length (Variables|/Game/Blueprint/Spline.Spline_C|GetSpawnableSplineCharacters (LocalVariables|GetCurrentSpline))) 1))
        (LocalVariables|SetSplineCharacterIndex 0)
        (else
          (Math|Integer|IncrementInt (LocalVariables|GetSplineCharacterIndex)))))
    (LocalVariables|SetCurrentDistance 0.0)))