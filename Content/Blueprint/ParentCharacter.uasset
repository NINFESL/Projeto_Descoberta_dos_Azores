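; Parent character Blueprint for movement constrained to a spline path, initializing its speed to walk speed on BeginPlay.
; AddMovement scales speed by an axis value to set acceleration and advances the distance along the spline using frame delta time.
; UpdateLocationAndRotation samples the referenced spline at that distance for world X, Y and rotation, preserving the actor's own Z so height is independent of the path.
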(event EventBeginPlay
  ;[1 1 1] Initialise Character
  (Variables|Default|SetCharacterSpeed (Variables|CharacterProperties|GetWalkSpeed)))

(fn ConstructionScript)

(fn AddMovement
  (bind _axisvalue (Variables|Default|GetAxisValue))
  (bind _characterspeed (Variables|Default|GetCharacterSpeed))
  (bind _returnvalue (* _characterspeed _axisvalue))
  (Variables|Default|SetPlayerAcceleration _returnvalue)
  (Variables|Default|SetDistanceAlongSpline (+ (Variables|Default|GetDistanceAlongSpline) (* _returnvalue (Utilities|Time|GetWorldDeltaSeconds)))))

(fn UpdateLocationandRotation
  (bind _splineref (Variables|CharacterProperties|GetSplineRef))
  (bind _distancealongspline (Variables|Default|GetDistanceAlongSpline))
  (bind _spline (Variables|/Game/Blueprint/Spline.Spline_C|GetSpline _splineref))
  (bind _returnvalue (Spline|GetLocationatDistanceAlongSpline _spline _distancealongspline "World"))
  (Transformation|SetActorLocationAndRotation (Math|Vector|MakeVector (.x _returnvalue) (.y _returnvalue) (.z (Transformation|GetActorLocation))) (Spline|GetRotationatDistanceAlongSpline (Variables|/Game/Blueprint/Spline.Spline_C|GetSpline (Variables|CharacterProperties|GetSplineRef)) (Variables|Default|GetDistanceAlongSpline) "World")))